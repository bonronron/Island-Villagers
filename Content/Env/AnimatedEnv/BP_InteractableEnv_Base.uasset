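; Base Blueprint for interactable environment objects that NPCs can use.
; Interaction prints a debug message naming the object and returns a fixed task enum value with animation data from the NPCAnimation variable.
; Simple getters expose the object's score through GetPlayerScore and its interactable flag.
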(fn `GetPlayerScore`
  (returns (ReturnValue :type "Float (single-precision)"))
  (return (`self.ObjectScore`)))

(fn `Interaction`
  (params (NPC :type "Actor Object Reference"))
  (returns (Task :type "/Game/Constants/Tasks Enum") (`Animation Data` :type "SingleAnimationPlayData Structure"))
  (`KismetSystemLibrary.PrintString` (`KismetStringLibrary.Concat_StrStr` "Interacting with" (`KismetSystemLibrary.GetObjectName` self)))
  (return "NewEnumerator3" (`SkeletalMeshComponent.AnimationData` (`self.NPC_Animation`))))

(fn `isInteractable?`
  (returns (isInteractable :type Boolean))
  (return (`self.IsInteractable`)))

(fn `UserConstructionScript`)