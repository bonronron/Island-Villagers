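; Base NPC Blueprint that the player can order to a location and that tracks nearby interactable environment objects.
; A move order writes the location and player override to the AI Blackboard, resets the current task and interactable object, and restores Animation Blueprint mode.
; InteractBox overlaps maintain a set of interactables, from which one is picked at random.
; A map stores efficiency per role type, defaulting to 100.
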(event `PlayerAskedToMoveTo`
  (params (WorldLocation :type "Vector Structure"))
  (bind _blackboard (`AIController.Blackboard` (`AIBlueprintHelperLibrary.GetAIController` self)))
  (`BlackboardComponent.SetValueAsVector` _blackboard "LocationOnMap" WorldLocation)
  (`BlackboardComponent.SetValueAsBool` _blackboard "PlayerOverride" true)
  (`BlackboardComponent.SetValueAsEnum` _blackboard "CurrentTask" 0)
  (`BlackboardComponent.SetValueAsObject` _blackboard "InteractableObject" null)
  (`SkeletalMeshComponent.SetAnimationMode` (`self.Mesh`) "AnimationBlueprint" true))

(event `self.InteractBox.OnComponentBeginOverlap`
  (params (OverlappedComponent :type "PrimitiveComponent Object Reference") (OtherActor :type "Actor Object Reference") (OtherComp :type "PrimitiveComponent Object Reference") (OtherBodyIndex :type Integer) (bFromSweep :type Boolean) (SweepResult :type "HitResult Structure (by ref)"))
  (bind _asbp_interactable_env_base (cast `/Game/Env/AnimatedEnv/BP_InteractableEnv_Base` OtherActor)
    (:`then`
      (`BlueprintSetLibrary.Set_Add` (`self.InteractableObjects`) _asbp_interactable_env_base))
    (:`CastFailed`
      (`KismetSystemLibrary.PrintString` (`KismetSystemLibrary.GetObjectName` OtherActor)))))

(event `self.InteractBox.OnComponentEndOverlap`
  (params (OverlappedComponent :type "PrimitiveComponent Object Reference") (OtherActor :type "Actor Object Reference") (OtherComp :type "PrimitiveComponent Object Reference") (OtherBodyIndex :type Integer))
  (bind _interactableobjects (`self.InteractableObjects`))
  (bind _asbp_interactable_env_base (cast `/Game/Env/AnimatedEnv/BP_InteractableEnv_Base` OtherActor))
  (if (`BlueprintSetLibrary.Set_Contains` _interactableobjects _asbp_interactable_env_base)
    (`BlueprintSetLibrary.Set_Remove` _interactableobjects _asbp_interactable_env_base)))

(event `/Game/NPCs/BPI_RoleEfficiency.SetEfficiencyOfType`
  (params (Type :type "/Game/Constants/NPC_Roles Enum" :default "NewEnumerator0") (Efficiency :type Integer))
  (`BlueprintMapLibrary.Map_Add` (`self.RoleEfficiency`) Type Efficiency))

(fn `GetEfficiencyOfType`
  (params (Type :type "/Game/Constants/NPC_Roles Enum" :default "NewEnumerator0"))
  (returns (Efficiency :type Integer))
  (bind (_value _returnvalue) (`BlueprintMapLibrary.Map_Find` (`self.RoleEfficiency`) Type))
  (if _returnvalue
    (return _value)
    (else
      (return 100))))

(fn `GetInteractionObject`
  (returns (OutItem :type "/Game/Env/AnimatedEnv/BP_InteractableEnv_Base Object Reference"))
  (bind _interactableobjects (`self.InteractableObjects`))
  (if (`BlueprintSetLibrary.Set_IsNotEmpty` _interactableobjects)
    (bind _result (`BlueprintSetLibrary.Set_ToArray` _interactableobjects)))
  (return (`KismetArrayLibrary.Array_Random` _result)))

(fn `UserConstructionScript`)